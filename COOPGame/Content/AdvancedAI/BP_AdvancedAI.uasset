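; BP_AdvancedAI is an AI-controlled actor that runs a behavior tree and displays its health.
; On BeginPlay, the server has its AI controller run BT_AdvancedAI.
; Every Tick writes HealthComp's health to the TextScore text, colored green at or above LowHealthThreshold and red below.
; Leftover blackboard setters, including one targeting the player pawn, are unconnected and never run.
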(event `self.ReceiveBeginPlay`
  (if (`self.HasAuthority`)
    (`AIController.RunBehaviorTree` (`AIBlueprintHelperLibrary.GetAIController` self) "/Game/AdvancedAI/BT_AdvancedAI.BT_AdvancedAI")))

(event `self.ReceiveTick`
  (params (DeltaSeconds :type "Float (single-precision)"))
  (bind _health (`SHealthComponent.Health` (`self.HealthComp`)))
  (`TextRenderComponent.K2_SetText` (`self.TextScore`) (`KismetTextLibrary.Conv_DoubleToText` _health "HalfToEven"))
  (`TextRenderComponent.SetTextRenderColor` (`self.TextScore`) (`KismetMathLibrary.Conv_LinearColorToColor` (`KismetMathLibrary.SelectColor` (struct :`G` 1.0 :`A` 1.0) (struct :`R` 1.0 :`A` 1.0) (>= _health (`self.LowHealthThreshold`))))))

(fn `UserConstructionScript`)