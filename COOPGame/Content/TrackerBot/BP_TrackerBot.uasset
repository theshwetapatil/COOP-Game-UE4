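; Tracker bot Blueprint with speed-driven audio and a debug view of the navigation path to the player.
; Tick maps velocity magnitude to the audio component's volume multiplier and prints that value on screen.
; FindNextPathPoint computes a synchronous path to the player pawn and only draws debug spheres at its points.
; BeginPlay is empty, and the SimpleMove and FindNextPathPoint calls in this graph are disconnected.
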(event `self.ReceiveBeginPlay`)

(event `FindNextPathPoint`
  (bind _returnvalue (`NavigationSystemV1.FindPathToActorSynchronously` (`self.K2_GetActorLocation`) (`GameplayStatics.GetPlayerPawn` 0) 50.0 null null))
  (for _array_element (`NavigationPath.PathPoints` _returnvalue)
    (`KismetSystemLibrary.DrawDebugSphere` _array_element 20.0 12 (struct :`R` 1.0 :`G` 0.879623 :`A` 1.0) 6.0 1.0)))

(event `self.ReceiveTick`
  (params (DeltaSeconds :type "Float (single-precision)"))
  (bind _returnvalue (`KismetMathLibrary.MapRangeClamped` (`KismetMathLibrary.VSize` (`self.GetVelocity`)) 10.0 1000.0 0.1 2.0))
  (`AudioComponent.SetVolumeMultiplier` (`self.AudioComp`) _returnvalue)
  (`KismetSystemLibrary.PrintString` (`KismetStringLibrary.Conv_DoubleToString` _returnvalue) true true (struct :`G` 0.66 :`B` 1.0 :`A` 1.0) 0.0))

(fn `UserConstructionScript`)